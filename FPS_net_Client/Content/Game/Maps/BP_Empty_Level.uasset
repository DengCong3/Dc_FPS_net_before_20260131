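; BP_Empty_Level is an actor Blueprint holding test scaffolding for a TCP client link between Unreal and a server.
; BeginPlay, Tick, the Connect, Send and Disconnect input actions, and the construction script are all empty.
; Detached node chains would connect using ServerIP and ServerPort, print received messages, send a fixed string, disconnect, and print hello messages.
; None of these chains is wired to an event, so none runs.
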(event `self.ReceiveBeginPlay`)

(event `Key|One`
  (params (Key :type "Key Structure")))

(event `EnhancedInput|/Game/Input/IA_TCP_Connect`
  (params (ActionValue :type Boolean) (ElapsedSeconds :type "Float (double-precision)") (TriggeredSeconds :type "Float (double-precision)") (InputAction :type "InputAction Object Reference" :default "/Game/Input/IA_TCP_Connect.IA_TCP_Connect")))

(event `EnhancedInput|/Game/Input/IA_TCP_Send`
  (params (ActionValue :type Boolean) (ElapsedSeconds :type "Float (double-precision)") (TriggeredSeconds :type "Float (double-precision)") (InputAction :type "InputAction Object Reference" :default "/Game/Input/IA_TCP_Send.IA_TCP_Send")))

(event `self.ReceiveTick`
  (params (DeltaSeconds :type "Float (single-precision)")))

(event `Key|Two`
  (params (Key :type "Key Structure")))

(event `Key|Three`
  (params (Key :type "Key Structure")))

(event `EnhancedInput|/Game/Input/IA_TCP_Disconnect`
  (params (ActionValue :type Boolean) (ElapsedSeconds :type "Float (double-precision)") (TriggeredSeconds :type "Float (double-precision)") (InputAction :type "InputAction Object Reference" :default "/Game/Input/IA_TCP_Disconnect.IA_TCP_Disconnect")))

(fn `UserConstructionScript`)