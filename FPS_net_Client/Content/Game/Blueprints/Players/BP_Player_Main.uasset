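; Local player Blueprint for a TCP multiplayer client test that mirrors player states received from the server.
; Debug keys connect to a localhost server, send a test message, disconnect and print the player ID.
; Tick polls TCP: "id" messages set and acknowledge MyPlayerID, while "pos" messages are parsed per player.
; The local entry teleports this actor; others update or spawn BP_Player_Other proxies tracked in OtherActorMap by ID.
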(event `self.ReceiveBeginPlay`)

(event `Key|One`
  (params (Key :type "Key Structure"))
  (:`Released`
    (`BPFL_TcpClient.ConnectToServer` "127.0.0.1" 8888)))

(event `Key|Two`
  (params (Key :type "Key Structure"))
  (:`Released`
    (`BPFL_TcpClient.SendTCPMessage` "Client Test from UE")))

(event `Key|Four`
  (params (Key :type "Key Structure"))
  (:`Released`
    (`KismetSystemLibrary.PrintString` (`KismetStringLibrary.Conv_IntToString` (`self.MyPlayerID`)))))

(event `Key|Three`
  (params (Key :type "Key Structure"))
  (:`Pressed`
    (`BPFL_TcpClient.DisconnectTCP`)
    (`KismetSystemLibrary.PrintString` "\"⚠️ 已主动断开服务器连接")))

(event `self.ReceiveTick`
  (params (DeltaSeconds :type "Float (single-precision)"))
  (bind _returnvalue (`BPFL_TcpClient.ReceiveTCPMessage`))
  (if (not (`KismetStringLibrary.IsEmpty` _returnvalue))
    (`KismetSystemLibrary.PrintString` _returnvalue true true (struct :`R` 0.420289 :`G` 0.344927 :`B` 1.0 :`A` 1.0))
    (if (`KismetStringLibrary.StartsWith` _returnvalue "pos")
      (bind (_outplayerdatas _bparsesuccess) (`BPFL_MessageParser.Parse_PosMessage` _returnvalue))
      (if _bparsesuccess
        (for _array_element _outplayerdatas
          (bind (_playerid _pos _rot _hp) (break `PlayerPosData` _array_element))
          (if (== _playerid (`self.MyPlayerID`))
            (`KismetSystemLibrary.PrintString` "true")
            (`KismetSystemLibrary.PrintString` (`KismetStringLibrary.Conv_RotatorToString` _rot))
            (`self.K2_SetActorLocation` _pos false true)
            (`self.K2_SetActorRotation` _rot true)
            (else
              (`KismetSystemLibrary.PrintString` "不相等")
              (bind (_value _returnvalue_2) (`BlueprintMapLibrary.Map_Find` (`self.OtherActorMap`) _playerid))
              (if _returnvalue_2
                (`KismetSystemLibrary.PrintString` "已经找到")
                (`/Game/Game/Blueprints/Players/BP_Player_Other.UpdatePlayerData` _value _pos _rot _hp)
                (else
                  (`KismetSystemLibrary.PrintString` "没有找到")
                  (bind _returnvalue_3 (`|SpawnActorFromClass` "/Game/Game/Blueprints/Players/BP_Player_Other.BP_Player_Other_C" (`KismetMathLibrary.MakeTransform` _pos _rot) "AlwaysSpawn" "MultiplyWithRoot" null _playerid _hp null))
                  (`/Game/Game/Blueprints/Players/BP_Player_Other.InitPlayerData` _returnvalue_3 _playerid)
                  (`BlueprintMapLibrary.Map_Add` (`self.OtherActorMap`) _playerid _returnvalue_3))))))
        (else
          (`KismetSystemLibrary.PrintString` "解析失败")))
      (elif (`KismetStringLibrary.StartsWith` _returnvalue "id")
        (bind _returnvalue_4 (`BPFL_TcpClient.GetPlayerID`))
        (bind _output_get (set `self.MyPlayerID` _returnvalue_4))
        (`KismetSystemLibrary.PrintString` (`KismetStringLibrary.Conv_IntToString` _output_get))
        (bind _returnvalue_5 (`KismetStringLibrary.Conv_IntToString` (`KismetSystemLibrary.MakeLiteralInt` _output_get)))
        (`BPFL_TcpClient.SendTCPMessage` (`KismetStringLibrary.Concat_StrStr` "用户id为:" _returnvalue_5 "的玩家已经在客户端设置Playerid并且回复消息"))
        (`KismetSystemLibrary.PrintString` _returnvalue_5)))))

(fn `UserConstructionScript`)