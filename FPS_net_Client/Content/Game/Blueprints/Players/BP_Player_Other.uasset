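; BP_Player_Other represents another player, mirroring position, rotation, HP and animation ID supplied from outside.
; InitPlayerData stores the player ID and initial animation ID; the event graph holds no active logic.
; UpdatePlayerData teleports the actor without sweep or interpolation, stores HP, and pushes the animation ID into AniBP_Net, printing an error if the cast fails.
; UpdatePlayerAni only stores the animation ID, without forwarding it to the anim instance.
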(fn `InitPlayerData`
  (params (InitID :type Integer) (aniid :type Integer))
  (set `self.OtherPlayerID` InitID)
  (set `self.ani_id` aniid))

(fn `UpdatePlayerAni`
  (params (anid :type Integer))
  (set `self.ani_id` anid))

(fn `UpdatePlayerData`
  (params (NewPos :type "Vector Structure") (NewRot :type "Rotator Structure") (NewHP :type Integer) (Newaniid :type Integer))
  (`self.K2_SetActorLocation` NewPos false true)
  (`self.K2_SetActorRotation` NewRot true)
  (set `self.CurrentHP` NewHP)
  (bind _output_get (set `self.ani_id` Newaniid))
  (bind _asani_bp_net (cast `/Game/Game/Blueprints/Players/AniBP_Net` (`SkeletalMeshComponent.GetAnimInstance` (`self.SkeletalMesh`)))
    (:`then`
      (set `/Game/Game/Blueprints/Players/AniBP_Net.ani_id` _output_get _asani_bp_net))
    (:`CastFailed`
      (`KismetSystemLibrary.PrintString` "寻找动画蓝图失败"))))

(fn `UserConstructionScript`)