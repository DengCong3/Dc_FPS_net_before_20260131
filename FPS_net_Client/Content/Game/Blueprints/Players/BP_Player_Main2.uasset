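; Local player Blueprint for a networked game client that sends input to a TCP server and takes its transform from it.
; Debug keys connect to or disconnect from localhost; movement keys, fire clicks and mouse-direction changes go out as short string commands.
; Tick reads queued messages, setting the player ID, applying position, rotation and animation ID, spawning or updating BP_Player_Other actors through an ID map, and printing status and death notices.
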(event `Key|LeftMouseButton`
  (params (Key :type "Key Structure"))
  (:`Pressed`
    (`BPFL_TcpClient.SendTCPMessage` "k|f"))
  (:`Released`
    (`BPFL_TcpClient.SendTCPMessage` "k|nf")))

(event `Key|W`
  (params (Key :type "Key Structure"))
  (:`Pressed`
    (`BPFL_TcpClient.SendTCPMessage` "k|1"))
  (:`Released`
    (`BPFL_TcpClient.SendTCPMessage` "k|m")))

(event `Key|A`
  (params (Key :type "Key Structure"))
  (:`Pressed`
    (`BPFL_TcpClient.SendTCPMessage` "k|3"))
  (:`Released`
    (`BPFL_TcpClient.SendTCPMessage` "k|p")))

(event `Key|S`
  (params (Key :type "Key Structure"))
  (:`Pressed`
    (`BPFL_TcpClient.SendTCPMessage` "k|2"))
  (:`Released`
    (`BPFL_TcpClient.SendTCPMessage` "k|n")))

(event `Key|D`
  (params (Key :type "Key Structure"))
  (:`Pressed`
    (`BPFL_TcpClient.SendTCPMessage` " k|4"))
  (:`Released`
    (`BPFL_TcpClient.SendTCPMessage` "k|q")))

(event `self.ReceiveBeginPlay`
  (bind _returnvalue (`GameplayStatics.GetPlayerController` 0))
  (`self.EnableInput` _returnvalue)
  (`PlayerController.SetViewTargetWithBlend` _returnvalue null 0.0 "VTBlend_Linear" 0.0 false))

(event `InputAxisKey|MouseY`
  (params (AxisValue :type "Float (single-precision)"))
  (bind _nowmouse_state (`self.nowmouse_state`))
  (bind _lastmouse_state (`self.lastmouse_state`))
  (if (< AxisValue 0.0)
    (bind _output_get (set `self.nowmouse_state` -1))
    (if (not (== _lastmouse_state _output_get))
      (set `self.lastmouse_state` _output_get)
      (if (== _nowmouse_state 0) :!label _label
        (`BPFL_TcpClient.SendTCPMessage` "m|s")
        (elif (== _nowmouse_state 1)
          (`BPFL_TcpClient.SendTCPMessage` "m|r")
          (else
            (`BPFL_TcpClient.SendTCPMessage` "m|l")))))
    (elif (== 0.0 AxisValue)
      (bind _output_get_2 (set `self.nowmouse_state` 0))
      (if (not (== _output_get_2 _lastmouse_state))
        (set `self.lastmouse_state` _output_get_2)
        (goto _label))
      (else
        (bind _output_get_3 (set `self.nowmouse_state` 1))
        (if (not (== _output_get_3 _lastmouse_state))
          (set `self.lastmouse_state` _output_get_3)
          (goto _label))))))

(event `Key|Four`
  (params (Key :type "Key Structure"))
  (:`Released`
    (`KismetSystemLibrary.PrintString` (`KismetStringLibrary.Conv_IntToString` (`self.MyPlayerID`)))))

(event `Key|Two`
  (params (Key :type "Key Structure"))
  (:`Released`
    (`BPFL_TcpClient.SendTCPMessage` "Client Test from UE")))

(event `Key|One`
  (params (Key :type "Key Structure"))
  (:`Released`
    (bind _returnvalue (`BPFL_TcpClient.ConnectToServer` "127.0.0.1" 8888))
    (if _returnvalue
      (set `self.bIsServerConnected` true)
      (`BPFL_TcpClient.StartAsyncReceive`))))

(event `Key|Three`
  (params (Key :type "Key Structure"))
  (:`Pressed`
    (`BPFL_TcpClient.DisconnectFromServer`)
    (set `self.bIsServerConnected` false)
    (`KismetSystemLibrary.PrintString` "已主动断开服务器连接")))

(event `sendheartbeat`
  (`BPFL_TcpClient.SendTCPMessage` "heartbeat|"))

(event `self.ReceiveTick`
  (params (DeltaSeconds :type "Float (single-precision)"))
  (if (`self.bIsServerConnected`)
    (bind (_outmessage _returnvalue) (`BPFL_TcpClient.GetQueuedMessage`))
    (if _returnvalue
      (`KismetSystemLibrary.PrintString` _outmessage true true (struct :`R` 0.420289 :`G` 0.344927 :`B` 1.0 :`A` 1.0))
      (if (`KismetStringLibrary.StartsWith` _outmessage "pos")
        (bind (_outplayerdatas _bparsesuccess) (`BPFL_MessageParser.Parse_PosMessage` _outmessage))
        (if _bparsesuccess
          (for _array_element _outplayerdatas
            (bind (_playerid _pos _rot _hp _ani_id) (break `PlayerPosData` _array_element))
            (if (== _playerid (`self.MyPlayerID`))
              (`KismetSystemLibrary.PrintString` "true")
              (`self.K2_SetActorLocation` _pos false true)
              (`self.K2_SetActorRotation` _rot true)
              (bind _output_get (set `self.ani_id` _ani_id))
              (bind _asani_bp_net (cast `/Game/Game/Blueprints/Players/AniBP_Net` (`SkeletalMeshComponent.GetAnimInstance` (`self.SkeletalMesh`)))
                (:`then`
                  (set `/Game/Game/Blueprints/Players/AniBP_Net.ani_id` _output_get _asani_bp_net))
                (:`CastFailed`
                  (`KismetSystemLibrary.PrintString` "转换失败")))
              (else
                (`KismetSystemLibrary.PrintString` "不相等")
                (bind (_value _returnvalue_2) (`BlueprintMapLibrary.Map_Find` (`self.OtherActorMap`) _playerid))
                (if _returnvalue_2
                  (`KismetSystemLibrary.PrintString` "已经找到")
                  (`/Game/Game/Blueprints/Players/BP_Player_Other.UpdatePlayerData` _value _pos _rot _hp _ani_id)
                  (else
                    (`KismetSystemLibrary.PrintString` "没有找到")
                    (bind _returnvalue_3 (`|SpawnActorFromClass` "/Game/Game/Blueprints/Players/BP_Player_Other.BP_Player_Other_C" (`KismetMathLibrary.MakeTransform` _pos _rot) "AlwaysSpawn" "MultiplyWithRoot" null _playerid _hp _ani_id null))
                    (`/Game/Game/Blueprints/Players/BP_Player_Other.InitPlayerData` _returnvalue_3 _playerid _ani_id)
                    (`BlueprintMapLibrary.Map_Add` (`self.OtherActorMap`) _playerid _returnvalue_3))))))
          (else
            (`KismetSystemLibrary.PrintString` "解析失败")))
        (elif (`KismetStringLibrary.StartsWith` _outmessage "id")
          (bind (_lefts _rights) (`KismetStringLibrary.Split` _outmessage "|"))
          (bind _output_get_2 (set `self.MyPlayerID` (`KismetStringLibrary.Conv_StringToInt` _rights)))
          (`KismetSystemLibrary.PrintString` (`KismetStringLibrary.Conv_IntToString` _output_get_2))
          (bind _returnvalue_4 (`KismetStringLibrary.Conv_IntToString` (`KismetSystemLibrary.MakeLiteralInt` _output_get_2)))
          (`BPFL_TcpClient.SendTCPMessage` (`KismetStringLibrary.Concat_StrStr` "用户id为:" _returnvalue_4 "的玩家已经在客户端设置Playerid并且回复消息"))
          (`KismetSystemLibrary.PrintString` _returnvalue_4)
          (elif (`KismetStringLibrary.StartsWith` _outmessage "s")
            (`KismetSystemLibrary.PrintString` _rights)
            (elif (`KismetStringLibrary.StartsWith` _outmessage "d")
              (`KismetSystemLibrary.PrintString` (`KismetStringLibrary.Concat_StrStr` _rights "：游戏阵亡")))))))))

(fn `UserConstructionScript`)