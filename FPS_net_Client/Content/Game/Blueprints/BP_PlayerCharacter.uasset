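; Player character Blueprint with a prototype fire action and debug output.
; BeginPlay adds a LogUI_Simple widget to the viewport, while Tick prints the capsule's forward vector.
; IA_Fire toggles ISFire and, on press, runs a debug-drawn Visibility trace from the right-hand socket along capsule forward, without using the hit.
; Key 1 only prints a server-connection message; leftover connection and logging nodes are unwired.
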(event `self.ReceiveBeginPlay`
  (bind _returnvalue (`|CreateWidget` "/Game/Game/UMG/LogUI_Simple.LogUI_Simple_C"))
  (bind _output_get (set `self.UI` _returnvalue))
  (`UserWidget.AddToViewport` _output_get 0))

(event `Key|One`
  (params (Key :type "Key Structure"))
  (:`Pressed`
    (`KismetSystemLibrary.PrintString` "\"UE尝试连接服务器\"")))

(event `Key|Two`
  (params (Key :type "Key Structure")))

(event `EnhancedInput|/Game/Input/IA_Fire`
  (params (ActionValue :type Boolean) (ElapsedSeconds :type "Float (double-precision)") (TriggeredSeconds :type "Float (double-precision)") (InputAction :type "InputAction Object Reference" :default "/Game/Input/IA_Fire.IA_Fire"))
  (bind _returnvalue (`SceneComponent.GetSocketLocation` (`self.CharacterMesh`) "HandGrip_R"))
  (bind _returnvalue_2 (+ _returnvalue (* (+ (`KismetMathLibrary.GetForwardVector` (`SceneComponent.K2_GetComponentRotation` (`self.CapsuleComponent`))) (0.0 0.0 0.0)) (1000.0 1000.0 1000.0))))
  (:`Started`
    (set `self.IS_Fire` true)
    (`KismetSystemLibrary.PrintString` (`KismetStringLibrary.Concat_StrStr` "\"打印:\"" (`KismetStringLibrary.Conv_VectorToString` _returnvalue_2)))
    (`KismetSystemLibrary.LineTraceSingle` :`Start` _returnvalue :`End` _returnvalue_2 :`TraceChannel` "TraceTypeQuery1" :`DrawDebugType` "ForDuration"))
  (:`Completed`
    (set `self.IS_Fire` false)))

(event `self.ReceiveTick`
  (params (DeltaSeconds :type "Float (single-precision)"))
  (`KismetSystemLibrary.PrintString` (`KismetStringLibrary.Conv_VectorToString` (+ (`KismetMathLibrary.GetForwardVector` (`SceneComponent.K2_GetComponentRotation` (`self.CapsuleComponent`))) (0.0 0.0 0.0)))))

(fn `UserConstructionScript`)